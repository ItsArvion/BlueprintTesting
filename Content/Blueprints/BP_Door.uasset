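; BP_Door is a locked sliding door that opens and closes on Interact once PickupKey has set its HasKey flag.
; A FlipFlop alternates playing and reversing a timeline that drives the door's relative Y location, with a sound at each toggle.
; Without the key, Interact shows a not-enough-keys prompt.
; Collider overlaps with the first-person character show and hide the press-E prompt.
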(event OnComponentBeginOverlap(Collider)
  (params (OverlappedComponent :type Primitive%20Component%20Object%20Reference) (OtherActor :type Actor%20Object%20Reference) (OtherComp :type Primitive%20Component%20Object%20Reference) (OtherBodyIndex :type Integer) (bFromSweep :type Boolean) (SweepResult :type Hit%20Result%20Structure%20%28by%20ref%29))
  (Utilities|Casting|CastToBP_FirstPersonCharacter OtherActor)
  (Rendering|SetVisibility (Variables|Default|Getpress%20e%20to%20interact) true false))

(event OnComponentEndOverlap(Collider)
  (params (OverlappedComponent :type Primitive%20Component%20Object%20Reference) (OtherActor :type Actor%20Object%20Reference) (OtherComp :type Primitive%20Component%20Object%20Reference) (OtherBodyIndex :type Integer))
  (Utilities|Casting|CastToBP_FirstPersonCharacter OtherActor)
  (Rendering|SetVisibility (Variables|Default|Getpress%20e%20to%20interact) false false))

(event EventInteract
  (if (Variables|Default|GethasKey?)
    (Rendering|SetVisibility (Variables|Default|Getnotenoughkeys) false false)
    (Utilities|FlowControl|FlipFlop
      (:A
        (Audio|PlaySoundatLocation "/Game/Sounds/dooropens_Cue.dooropens_Cue" (Transformation|GetActorLocation) "0, 0, 0" 1.0 1.0 0.0 "/Game/Blueprints/SoundAttenuation.SoundAttenuation" 0 0 0)
        (bind _doortrack (Timeline|TL_DoorTimeline Play)
          (:Update
            (Transformation|SetRelativeLocation (Variables|Default|Getdoor) (Math|Vector|MakeVector 0.0 _doortrack 0.0) false false))))
      (:B
        (Audio|PlaySoundatLocation "/Game/Sounds/dooropens.dooropens" (Transformation|GetActorLocation) "0, 0, 0" 1.0 1.0 0.0 0 0 0 0)
        (Timeline|TL_DoorTimeline Reverse)))
    (else
      (Rendering|SetVisibility (Variables|Default|Getnotenoughkeys) true false))))

(event EventPickupKey
  (Variables|Default|SethasKey? true))

(fn ConstructionScript)