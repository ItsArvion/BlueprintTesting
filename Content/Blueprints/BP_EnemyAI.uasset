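; Enemy character Blueprint that chases the player on sight and attacks with a sword, turning periodically when no player is seen.
; PawnSensing briefly sets a sight flag that Tick polls to run AI MoveTo or the delayed turn.
; Reaching the player plays a slash montage, gated by a montage-length cooldown.
; TriggerSword starts a looping timer that line-traces between sword sockets and applies damage until stopTriggerSword clears it.
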(event OnSeePawn(PawnSensing)
  (params (Pawn :type Pawn%20Object%20Reference))
  (Variables|Default|SetisSeeingPlayer? true)
  (Utilities|FlowControl|Delay 0.01)
  (Variables|Default|SetisSeeingPlayer? false))

(event Custom|followPlayer
  (if (Variables|Default|GetisSeeingPlayer?)
    (AI|AIMoveTo self "0, 0, 0" (Game|GetPlayerCharacter 0) 1e+01 false
      (:OnSuccess
        (if (Variables|Default|GetcanAttack?)
          (Variables|Default|SetcanAttack? false)
          (Development|PrintString "Cannot attack")
          (bind _returnvalue (Animation|PlayAnimMontage "/Game/Animations/AI/Sword_And_Shield_Slash_Anim_Montage.Sword_And_Shield_Slash_Anim_Montage" 1.0 "None"))
          (Utilities|FlowControl|Delay (+ _returnvalue 1.0))
          (Variables|Default|SetcanAttack? true)
          (Development|PrintString "Can attack"))))))

(event Custom|TriggerSword
  (bind _returnvalue (Utilities|Time|SetTimerbyEvent (delegate Custom|SwordLineTrace) 0.01 true))
  (Variables|Default|SettriggerSwordEvent _returnvalue))

(event Custom|SwordLineTrace
  (bind _outhit (Collision|LineTraceByChannel (Transformation|GetSocketLocation (Variables|Default|GetSword) "Start") (Transformation|GetSocketLocation (Variables|Default|GetSword) "End") "TraceTypeQuery2" false 0 "ForDuration"))
  (Game|Damage|ApplyDamage (.HitActor (Collision|BreakHitResult _outhit)) 1e+01 0 0))

(event Custom|stopTriggerSword
  (Utilities|Time|ClearandInvalidateTimerbyHandle (Variables|Default|GettriggerSwordEvent)))

(event EventBeginPlay
  (Variables|Default|SetcanAttack? true))

(event EventTick
  (params (DeltaSeconds :type Float%20%28single-precision%29))
  (if (Variables|Default|GetisSeeingPlayer?)
    (CallFunction|FollowPlayer)
    (else
      (Utilities|FlowControl|Delay 5.0)
      (Transformation|SetActorRotation (Math|Rotator|MakeRotator 0.0 0.0 (+ (.yaw (Transformation|GetActorRotation)) 9e+01))))))

(fn ConstructionScript)