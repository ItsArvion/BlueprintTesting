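; BP_Key is a pickup key actor that is linked to a Door.
; Interacting calls the door's PickupKeyMessage, plays a pickup sound and destroys the key.
; A sphere overlap shows its widget while the first-person character is nearby, and the widget is hidden shortly after BeginPlay.
; Hits play an attenuated metal clink, though the SoundPlaying guard resets immediately, so it does not throttle repeats.
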(event OnComponentHit(Key)
  (params (HitComponent :type Primitive%20Component%20Object%20Reference) (OtherActor :type Actor%20Object%20Reference) (OtherComp :type Primitive%20Component%20Object%20Reference) (NormalImpulse :type Vector :default "0, 0, 0") (Hit :type Hit%20Result%20Structure%20%28by%20ref%29))
  (if (not (Variables|Default|GetSound%20playing))
    (Variables|Default|SetSound%20playing true)
    (Audio|PlaySoundatLocation "/Game/Sounds/metalclink.metalclink" (Transformation|GetActorLocation) "0, 0, 0" 1.0 1.0 0.0 "/Game/Blueprints/SoundAttenuation.SoundAttenuation" 0 0 0)
    (Variables|Default|SetSound%20playing false)))

(event OnComponentBeginOverlap(Sphere)
  (params (OverlappedComponent :type Primitive%20Component%20Object%20Reference) (OtherActor :type Actor%20Object%20Reference) (OtherComp :type Primitive%20Component%20Object%20Reference) (OtherBodyIndex :type Integer) (bFromSweep :type Boolean) (SweepResult :type Hit%20Result%20Structure%20%28by%20ref%29))
  (Utilities|Casting|CastToBP_FirstPersonCharacter OtherActor)
  (Rendering|SetVisibility (Variables|Default|GetWidget) true false))

(event OnComponentEndOverlap(Sphere)
  (params (OverlappedComponent :type Primitive%20Component%20Object%20Reference) (OtherActor :type Actor%20Object%20Reference) (OtherComp :type Primitive%20Component%20Object%20Reference) (OtherBodyIndex :type Integer))
  (Utilities|Casting|CastToBP_FirstPersonCharacter OtherActor)
  (Rendering|SetVisibility (Variables|Default|GetWidget) false false))

(event EventBeginPlay
  (Utilities|FlowControl|Delay 0.1)
  (Rendering|SetVisibility (Variables|Default|GetWidget) false false))

(event EventInteract
  (Class|BPIDoor|PickupKey(Message) (Variables|Default|GetDoor))
  (Audio|PlaySoundatLocation "/Game/Sounds/pickup.pickup" (Transformation|GetActorLocation) "0, 0, 0" 1.0 1.0 0.0 0 0 0 0)
  (Actor|DestroyActor))

(fn ConstructionScript)