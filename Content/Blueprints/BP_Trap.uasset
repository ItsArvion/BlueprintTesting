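; BP_Trap is a single-use trap actor that explodes when an enemy AI walks into it.
; Its Box overlap deals damage to the BP_EnemyAI and spawns an explosion emitter at the trap.
; It then removes its cube meshes and trigger, waits briefly, updates the first-person character's trap deployed and destroyed flags, and destroys itself.
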(event OnComponentBeginOverlap(Box)
  (params (OverlappedComponent :type Primitive%20Component%20Object%20Reference) (OtherActor :type Actor%20Object%20Reference) (OtherComp :type Primitive%20Component%20Object%20Reference) (OtherBodyIndex :type Integer) (bFromSweep :type Boolean) (SweepResult :type Hit%20Result%20Structure%20%28by%20ref%29))
  (bind _asbp_enemy_ai (Utilities|Casting|CastToBP_EnemyAI OtherActor))
  (Game|Damage|ApplyDamage _asbp_enemy_ai 2e+01 0 0 "/Script/Engine.DamageType")
  (Effects|SpawnEmitteratLocation "/Game/StarterContent/Particles/P_Explosion.P_Explosion" (Transformation|GetActorLocation))
  (bind _asbp_first_person_character (Utilities|Casting|CastToBP_FirstPersonCharacter (Game|Player|GetPlayerPawn 0)))
  (Components|DestroyComponent (Variables|Default|GetCube_Material_002_0))
  (Utilities|FlowControl|Delay 2.0)
  (Variables|/Game/Blueprints/BP_FirstPersonCharacter.BP_FirstPersonCharacter_C|Settrapdeployed? _asbp_first_person_character false)
  (Variables|/Game/Blueprints/BP_FirstPersonCharacter.BP_FirstPersonCharacter_C|Settrap%20destroyed? _asbp_first_person_character true)
  (Actor|DestroyActor))

(event EventBeginPlay)

(event EventTick
  (params (DeltaSeconds :type Float%20%28single-precision%29)))

(fn ConstructionScript)