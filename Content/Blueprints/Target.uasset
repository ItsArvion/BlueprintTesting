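; Target actor that reacts visually when something overlaps its Sphere component.
; Begin overlap sets IsColliding, swaps the Cube to a brick material and plays a timeline that drives the Cube's relative scale.
; End overlap clears the flag, applies BaseMaterial and reverses the same timeline to animate the scale back.
; Overlaps are not filtered by actor, and IsColliding is only written in this graph.
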(event OnComponentBeginOverlap(Sphere)
  (params (OverlappedComponent :type Primitive%20Component%20Object%20Reference) (OtherActor :type Actor%20Object%20Reference) (OtherComp :type Primitive%20Component%20Object%20Reference) (OtherBodyIndex :type Integer) (bFromSweep :type Boolean) (SweepResult :type Hit%20Result%20Structure%20%28by%20ref%29))
  (Variables|Default|SetisColliding true)
  (Rendering|Material|SetMaterial (Variables|Default|GetCube) 0 "/Game/StarterContent/Materials/M_Brick_Clay_Beveled.M_Brick_Clay_Beveled")
  (bind _scale (Timeline|TL_CubeAnimation Play)
    (:Update
      (Transformation|SetRelativeScale3D (Variables|Default|GetCube) (Math|Conversions|ToVector(Float) _scale)))))

(event OnComponentEndOverlap(Sphere)
  (params (OverlappedComponent :type Primitive%20Component%20Object%20Reference) (OtherActor :type Actor%20Object%20Reference) (OtherComp :type Primitive%20Component%20Object%20Reference) (OtherBodyIndex :type Integer))
  (Variables|Default|SetisColliding false)
  (Rendering|Material|SetMaterial (Variables|Default|GetCube) 0 "/Game/FPWeapon/Materials/BaseMaterial.BaseMaterial")
  (bind _scale (Timeline|TL_CubeAnimation Reverse)
    (:Update
      (Transformation|SetRelativeScale3D (Variables|Default|GetCube) (Math|Conversions|ToVector(Float) _scale)))))

(fn ConstructionScript)